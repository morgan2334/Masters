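; Enemy character with a health bar widget, destroyed at zero health, that picks between greatsword, projectile, dive-roll and spin attacks.
; Attack makes a weighted random pick, with montage notifies triggering sphere-trace damage or projectile spawns.
; Tick tracks hit rates, which reweight three attacks after ten attempts to favour what lands.
; Player distance then resets projectile and roll weights each tick, overriding the projectile's hit-rate weight except at exactly the threshold.
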(event EventBeginPlay
  (Utilities|FlowControl|Sequence
    (:then_0
      (bind _asenemy_health_widget (Utilities|Casting|CastToEnemyHealthWidget (UserInterface|GetUserWidgetObject (Variables|Default|GetHealthBar))))
      (bind _output_get (Variables|Default|SetHealthBarRef _asenemy_health_widget))
      (Variables|/Game/Masters/Blueprints/Enemy/EnemyHealthWidget.EnemyHealthWidget_C|SetHealth _output_get 1e+02))
    (:then_1
      (Rendering|SetVisibility (Variables|Default|GetHealthBar) true false))))

(event EventAttack
  (bind _attack1pos (Variables|Default|GetAttack1Pos))
  (bind _attackspinpos (Variables|Default|GetAttackSpinPos))
  (bind _returnvalue (Transformation|GetWorldLocation _attackspinpos))
  (bind _returnvalue_2 (Transformation|GetWorldLocation _attack1pos))
  (Variables|Default|SetTimesAttacked (+ (Variables|Default|GetTimesAttacked) 1))
  (bind _sum_of_values (CallFunction|SumValues))
  (bind _indexthatwon (CallFunction|DetermineIndex (Math|Random|RandomFloatinRange 0.0 _sum_of_values)))
  (switch int (Math|Float|Truncate _indexthatwon)
    (:0
      ;[1 1 1] Attack
      (if (not (Variables|Default|GetIsAttacking))
        (Development|PrintString "attacking")
        (Variables|Default|SetAttack%200%20Amount (+ (Variables|Default|GetAttack%200%20Amount) 1.0))
        (Animation|Montage|PlayMontage (Variables|Character|GetMesh) "/Game/Masters/Blueprints/ANIM_Greatsword_Attack_01_Montage.ANIM_Greatsword_Attack_01_Montage"
          (:then
            (Variables|Default|SetIsAttacking true))
          (:OnCompleted
            (Utilities|FlowControl|Delay 0.5)
            (Variables|Default|SetIsAttacking false))
          (:OnNotifyBegin
            (bind (_outhit _returnvalue_3) (Collision|SphereTraceForObjects _returnvalue_2 (+ _returnvalue_2 (* (Math|Vector|GetForwardVector (Transformation|GetWorldRotation _attack1pos)) 2.5e+02)) 35.0 (Utilities|Array|MakeArray "ObjectTypeQuery3") false 0 "ForDuration"))
            (if _returnvalue_3
              (Game|Damage|ApplyDamage (.HitActor (Collision|BreakHitResult _outhit)) 1e+01 0 0)
              (Variables|Default|SetAttack%200%20Hits (+ (Variables|Default|GetAttack%200%20Hits) 1.0)))))))
    (:1
      ;[1 1 1] Ranged attack
      (if (not (Variables|Default|GetIsAttacking))
        (Development|PrintString "attacking 1")
        (Animation|Montage|PlayMontage (Variables|Character|GetMesh) "/Game/Masters/Blueprints/EvenBetterRangedMontage.EvenBetterRangedMontage"
          (:then
            (Variables|Default|SetIsAttacking true))
          (:OnCompleted
            (Utilities|FlowControl|Delay 0.5)
            (Variables|Default|SetIsAttacking false))
          (:OnNotifyBegin
            (Game|SpawnActorfromClass "/Game/Masters/Blueprints/Enemy/EnemyProjectile.EnemyProjectile_C" (Transformation|GetWorldTransform (Variables|Default|GetProjectilePos)) "Undefined" 0 0)
            (Variables|Default|SetTimesProjectileAttacked (+ (Variables|Default|GetTimesProjectileAttacked) 1.0))))))
    (:2
      (if (not (Variables|Default|GetIsAttacking))
        (Development|PrintString "attacking 2")
        (Animation|Montage|PlayMontage (Variables|Character|GetMesh) "/Game/Masters/Blueprints/ANIM_DiveRoll_Montage.ANIM_DiveRoll_Montage"
          (:then
            (Variables|Default|SetIsAttacking true))
          (:OnCompleted
            (Utilities|FlowControl|Delay 0.5)
            (Variables|Default|SetIsAttacking false)))))
    (:3
      (if (not (Variables|Default|GetIsAttacking))
        (Development|PrintString "attacking 3")
        (Variables|Default|SetTimesSwingAttacked (+ (Variables|Default|GetTimesSwingAttacked) 1.0))
        (Animation|Montage|PlayMontage (Variables|Character|GetMesh) "/Game/Masters/Blueprints/BOSSspin.BOSSspin"
          (:then
            (Variables|Default|SetIsAttacking true))
          (:OnCompleted
            (Utilities|FlowControl|Delay 0.5)
            (Variables|Default|SetIsAttacking false))
          (:OnNotifyBegin
            (bind (_outhit_2 _returnvalue_4) (Collision|SphereTraceForObjects _returnvalue (+ _returnvalue (* (Math|Vector|GetForwardVector (Transformation|GetWorldRotation _attackspinpos)) 2.5e+02)) 35.0 (Utilities|Array|MakeArray "ObjectTypeQuery3") false 0 "ForDuration"))
            (if _returnvalue_4
              (Game|Damage|ApplyDamage (.HitActor (Collision|BreakHitResult _outhit_2)) 1e+01 0 0)
              (Variables|Default|SetSwingAttackHits (+ (Variables|Default|GetSwingAttackHits) 1.0)))))))))

(event EventTick
  (params (DeltaSeconds :type Float%20%28single-precision%29))
  (Utilities|FlowControl|Sequence
    (:then_0
      ;[1 1 1] Mesures player distance
      (bind _outactors (Actor|GetAllActorsOfClass "/Game/ThirdPerson/Blueprints/BP_ThirdPersonCharacter.BP_ThirdPersonCharacter_C"))
      (Variables|Default|SetPlayer%20Distance (Math|Vector|Distance(Vector) (Transformation|GetActorLocation self) (Transformation|GetActorLocation (Utilities|Array|Get(acopy) _outactors)))))
    (:then_1
      ;[1 1 1] HitPercentageCalculations
      (Variables|Default|SetAttack%200%20Percent (* (/ (Variables|Default|GetAttack%200%20Hits) (Variables|Default|GetAttack%200%20Amount)) 1e+02)))
    (:then_2
      (Variables|Default|SetSwingAttackPercent (* (/ (Variables|Default|GetSwingAttackHits) (Variables|Default|GetTimesSwingAttacked)) 1e+02)))
    (:then_3
      (Variables|Default|SetProjectile%20hit%20percentage (* (/ (Variables|Default|GetTimesProjectileHit) (Variables|Default|GetTimesProjectileAttacked)) 1e+02)))
    (:then_4
      (if (> (Variables|Default|GetTimesAttacked) 10)
        (CallFunction|PercentageMode)))
    (:then_5
      (if (> (Variables|Default|GetPlayer%20Distance) 6e+02)
        (Utilities|Array|SetArrayElem (Variables|Default|GetWeightValues) 2 1.0)
        (Utilities|Array|SetArrayElem (Variables|Default|GetWeightValues) 1 1e+01)))
    (:then_6
      (if (< (Variables|Default|GetPlayer%20Distance) 6e+02)
        (Utilities|Array|SetArrayElem (Variables|Default|GetWeightValues) 2 2.0)
        (Utilities|Array|SetArrayElem (Variables|Default|GetWeightValues) 1 1.0)
        (Utilities|FlowControl|DoOnce false
          (:Completed
            (Development|PrintString "updated index")))))))

(event Game|Damage|EventAnyDamage
  (params (Damage :type Float%20%28single-precision%29) (DamageType :type Damage%20Type%20Object%20Reference) (InstigatedBy :type Controller%20Object%20Reference) (DamageCauser :type Actor%20Object%20Reference))
  ;[1 1 1] Recive Damage
  (Utilities|FlowControl|Delay 0.2)
  (bind _output_get (Variables|Default|SetHealth (Math|Float|Clamp(Float) (- (Variables|Default|GetHealth) Damage) 0.0 1e+02)))
  (Variables|/Game/Masters/Blueprints/Enemy/EnemyHealthWidget.EnemyHealthWidget_C|SetHealth (Variables|Default|GetHealthBarRef) _output_get)
  (if (== (Variables|Default|GetHealth) 0.0)
    (Actor|DestroyActor)
    (else
      (Development|PrintString "hit"))))

(fn ConstructionScript)

(fn SumValues
  (for _array_element (Variables|Default|GetWeightValues)
    (LocalVariables|SetLocalSum (+ _array_element (LocalVariables|GetLocalSum))))
  (return (LocalVariables|GetLocalSum)))

(fn DetermineIndex
  (params (Random%20value :type Float%20%28double-precision%29))
  (bind (_array_element _array_index) (Utilities|Array|ForEachLoopwithBreak (Variables|Default|GetWeightValues) :!label _label)
    (:LoopBody
      (bind _output_get (LocalVariables|SetLocalSum (+ _array_element (LocalVariables|GetLocalSum))))
      (if (>= _output_get Random%20value)
        (goto _label Break)))
    (:Completed
      (return (Math|Conversions|ToFloat(Integer) _array_index)))))

(fn PercentageMode
  (bind _weightvalues (Variables|Default|GetWeightValues))
  (Utilities|Array|SetArrayElem _weightvalues 0 (Math|Float|Clamp(Float) (Variables|Default|GetAttack%200%20Percent) 1e+01 1e+02))
  (Utilities|Array|SetArrayElem _weightvalues 1 (Math|Float|Clamp(Float) (Variables|Default|GetProjectile%20hit%20percentage) 1e+01 1e+02))
  (Utilities|Array|SetArrayElem _weightvalues 3 (Math|Float|Clamp(Float) (Variables|Default|GetSwingAttackPercent) 1e+01 1e+02)))